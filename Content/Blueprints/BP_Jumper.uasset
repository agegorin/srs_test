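; BP_Jumper is a jump pad that launches the third-person player character when it overlaps the pad's box collision.
; On overlap it calls Jump and adds JumpVelocity, rotated by the Arrow component's world rotation, to the character's current movement velocity, so the arrow orients the launch.
; It also plays the JumperUp timeline, which moves the Jumper component's relative height between set minimum and maximum positions.
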(event `self.BoxCollision.OnComponentBeginOverlap`
  (params (OverlappedComponent :type "PrimitiveComponent Object Reference") (OtherActor :type "Actor Object Reference") (OtherComp :type "PrimitiveComponent Object Reference") (OtherBodyIndex :type Integer) (bFromSweep :type Boolean) (SweepResult :type "HitResult Structure (by ref)"))
  (bind _asbp_third_person_character (cast `/Game/ThirdPerson/Blueprints/BP_ThirdPersonCharacter` OtherActor))
  (`|ExecutionSequence`
    (:`then_0`
      ;[1 1 1] Отправляем игрока в полет
      (`Character.Jump` _asbp_third_person_character)
      (bind _charactermovement (`Character.CharacterMovement` _asbp_third_person_character))
      (set `MovementComponent.Velocity` (+ (`KismetMathLibrary.GreaterGreater_VectorRotator` (`self.JumpVelocity`) (`SceneComponent.K2_GetComponentRotation` (`self.Arrow`))) (`MovementComponent.Velocity` _charactermovement)) _charactermovement))
    (:`then_1`
      ;[1 1 1] Анимация джамп-пада
      (bind (_direction _heightpos) (`Timeline|JumperUp` :!via `PlayFromStart`)
        (:`Update`
          (`SceneComponent.K2_SetRelativeLocation` (`self.Jumper`) (`KismetMathLibrary.MakeVector` 0.0 0.0 (`KismetMathLibrary.Lerp` (`self.MinJumperPos`) (`self.MaxJmperPos`) _heightpos)) false false))))))

(fn `UserConstructionScript`)