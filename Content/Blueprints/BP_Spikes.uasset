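; Spike trap that kills BP_ThirdPersonCharacter when it touches the moving DeathCollision.
; Entering TriggerCollision starts a delay timer, then a timeline drives DeathCollision's relative Z to extend the spikes.
; After a second delay, another timeline retracts them and either fires again immediately if the player is still inside or rearms.
; An Activated flag blocks re-triggering during a cycle.
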(event `self.TriggerCollision.OnComponentBeginOverlap`
  (params (OverlappedComponent :type "PrimitiveComponent Object Reference") (OtherActor :type "Actor Object Reference") (OtherComp :type "PrimitiveComponent Object Reference") (OtherBodyIndex :type Integer) (bFromSweep :type Boolean) (SweepResult :type "HitResult Structure (by ref)"))
  ;[1 1 1] Игрок запускает ловушку
  (cast `/Game/ThirdPerson/Blueprints/BP_ThirdPersonCharacter` OtherActor)
  (set `self.PlayerInTriggerCollision` true)
  (if (not (`self.Activated`))
    (`KismetSystemLibrary.K2_SetTimerDelegate` (delegate `SpikeOut_Event`) (`self.TriggeringTime`))
    (set `self.Activated` true)))

(event `SpikeOut_Event`
  ;[1 1 1] Ловушка выпускает шипы
  (bind (_direction _heightpos) (`Timeline|MoveDeathTimeline` :!via `PlayFromStart`)
    (:`Update`
      (`SceneComponent.K2_SetRelativeLocation` (`self.DeathCollision`) (`KismetMathLibrary.MakeVector` 0.0 0.0 _heightpos) false false))
    (:`Finished`
      (`KismetSystemLibrary.K2_SetTimerDelegate` (delegate `DisableSpikes_Event`) (`self.DisablingTime`)))))

(event `DisableSpikes_Event`
  ;[1 1 1] Ловушка убирает шипы
  (bind (_direction _heightpos) (`Timeline|DisableSpikesTimeline` :!via `PlayFromStart`)
    (:`Update`
      (`SceneComponent.K2_SetRelativeLocation` (`self.DeathCollision`) (`KismetMathLibrary.MakeVector` 0.0 0.0 _heightpos) false false))
    (:`Finished`
      ;[1 1 1] Если игрок все еще в зоне ловушки, то снова выпускаем шипы
      (if (`self.PlayerInTriggerCollision`)
        (`self.SpikeOut_Event`)
        (else
          (set `self.Activated` false))))))

(event `self.DeathCollision.OnComponentBeginOverlap`
  (params (OverlappedComponent :type "PrimitiveComponent Object Reference") (OtherActor :type "Actor Object Reference") (OtherComp :type "PrimitiveComponent Object Reference") (OtherBodyIndex :type Integer) (bFromSweep :type Boolean) (SweepResult :type "HitResult Structure (by ref)"))
  ;[1 1 1] Игрок натыкается на шипы
  (bind _asbp_third_person_character (cast `/Game/ThirdPerson/Blueprints/BP_ThirdPersonCharacter` OtherActor))
  (`/Game/ThirdPerson/Blueprints/BP_ThirdPersonCharacter.Death_Event` _asbp_third_person_character))

(event `self.TriggerCollision.OnComponentEndOverlap`
  (params (OverlappedComponent :type "PrimitiveComponent Object Reference") (OtherActor :type "Actor Object Reference") (OtherComp :type "PrimitiveComponent Object Reference") (OtherBodyIndex :type Integer))
  ;[1 1 1] Игрок покинул зону взаимодействия с триггером
  (cast `/Game/ThirdPerson/Blueprints/BP_ThirdPersonCharacter` OtherActor)
  (set `self.PlayerInTriggerCollision` false))

(fn `UserConstructionScript`)